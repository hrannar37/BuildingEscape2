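; Blueprint actor that moves the first puzzle's stairs vertically in response to FirstPuzzleMovingStairs down and up requests.
; It stores its start location at BeginPlay, and the StairMovement timeline offsets Z by a track-scaled multiple of the absolute starting height.
; A down request plays the timeline only if the computed Z is at or above a fixed threshold, otherwise stopping it.
; An up request reverses it.
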(event OnDownRequest(FirstPuzzleMovingStairs)
  (if (<= -33.0 (+ (* (Math|Float|Absolute(Float) (.Z (Math|Vector|BreakVector (stale EventBeginPlay _output_get)))) (stale _newtrack_0)) (.Z (Math|Vector|BreakVector (stale EventBeginPlay _output_get)))))
    (bind _newtrack_0 (Timeline|StairMovement Play)
      (:Update
        (Transformation|SetActorLocation (Math|Vector|MakeVector (.X (Math|Vector|BreakVector (stale EventBeginPlay _output_get))) (.Y (Math|Vector|BreakVector (stale EventBeginPlay _output_get))) (+ (* (Math|Float|Absolute(Float) (.Z (Math|Vector|BreakVector (stale EventBeginPlay _output_get)))) _newtrack_0) (.Z (Math|Vector|BreakVector (stale EventBeginPlay _output_get))))) false false)))
    (else
      (Timeline|StairMovement Stop))))

(event OnUpRequest(FirstPuzzleMovingStairs)
  (bind _newtrack_0 (Timeline|StairMovement Reverse)
    (:Update
      (Transformation|SetActorLocation (Math|Vector|MakeVector (.X (Math|Vector|BreakVector (stale EventBeginPlay _output_get))) (.Y (Math|Vector|BreakVector (stale EventBeginPlay _output_get))) (+ (* (Math|Float|Absolute(Float) (.Z (Math|Vector|BreakVector (stale EventBeginPlay _output_get)))) _newtrack_0) (.Z (Math|Vector|BreakVector (stale EventBeginPlay _output_get))))) false false))))

(event EventBeginPlay
  (bind _output_get (Variables|Default|SetInitialLocation (Transformation|GetActorLocation))))

(fn ConstructionScript)