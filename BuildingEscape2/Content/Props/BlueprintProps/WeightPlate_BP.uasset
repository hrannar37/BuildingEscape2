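; Weight plate prop that detects when the objects resting on it add up to a required weight.
; On every begin or end overlap of its collision box, it recalculates the total mass of all overlapping components.
; When the rounded total exactly equals WeightNeeded, it plays a 2D collapse sound and triggers nothing else.
; At BeginPlay it prints the text of its WeightNumber component.
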(event OnComponentBeginOverlap(WeightCollisionBox)
  (params (OverlappedComponent :type Primitive%20Component%20Object%20Reference) (OtherActor :type Actor%20Object%20Reference) (OtherComp :type Primitive%20Component%20Object%20Reference) (OtherBodyIndex :type Integer) (bFromSweep :type Boolean) (SweepResult :type Hit%20Result%20Structure%20%28by%20ref%29))
  (Variables|Default|SetTotal%20Weight%20On%20Plate 0.0)
  (for _array_element (Class|PrimitiveComponent|GetOverlappingComponents (Variables|Default|GetWeightCollisionBox))
    (Variables|Default|SetTotal%20Weight%20On%20Plate (+ (Physics|GetMass _array_element) (Variables|Default|GetTotal%20Weight%20On%20Plate))))
  (if (== (Math|Float|Round (Variables|Default|GetTotal%20Weight%20On%20Plate)) (Variables|Default|GetWeight%20Needed))
    (Audio|PlaySound2D "/Game/StarterContent/Audio/Collapse_Cue.Collapse_Cue")))

(event OnComponentEndOverlap(WeightCollisionBox)
  (params (OverlappedComponent :type Primitive%20Component%20Object%20Reference) (OtherActor :type Actor%20Object%20Reference) (OtherComp :type Primitive%20Component%20Object%20Reference) (OtherBodyIndex :type Integer))
  (Variables|Default|SetTotal%20Weight%20On%20Plate 0.0)
  (for _array_element (Class|PrimitiveComponent|GetOverlappingComponents (Variables|Default|GetWeightCollisionBox))
    (Variables|Default|SetTotal%20Weight%20On%20Plate (+ (Physics|GetMass _array_element) (Variables|Default|GetTotal%20Weight%20On%20Plate))))
  (if (== (Math|Float|Round (Variables|Default|GetTotal%20Weight%20On%20Plate)) (Variables|Default|GetWeight%20Needed))
    (Audio|PlaySound2D "/Game/StarterContent/Audio/Collapse_Cue.Collapse_Cue")))

(event EventBeginPlay
  (Development|PrintText (Variables|/Script/Engine.TextRenderComponent|GetText (Variables|Default|GetWeight%20Number))))

(event Collision|EventActorBeginOverlap
  (params (OtherActor :type Actor%20Object%20Reference)))

(event EventTick
  (params (DeltaSeconds :type Float%20%28single-precision%29)))

(fn ConstructionScript)