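; Pressable button prop that the player activates with the Use input while standing inside its trigger box.
; It enables input for the first player controller on BeginPlay and checks the player character's overlap on each press.
; A timeline animates the button mesh along its local Y position, then plays a sound at the base and fires ButtonPressed.
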(event EventBeginPlay
  (Input|EnableInput (Game|GetPlayerController 0)))

(event Collision|EventActorBeginOverlap
  (params (OtherActor :type Actor%20Object%20Reference)))

(event EventTick
  (params (DeltaSeconds :type Float%20%28single-precision%29)))

(event Input|ActionEvents|InputActionUse
  (params (Key :type Key%20Structure))
  (bind _button (Variables|Default|GetButton))
  (bind _returnvalue (Transformation|GetRelativeTransform _button))
  (bind _location (Math|Transform|BreakTransform _returnvalue))
  (bind (_x _y _z) (Math|Vector|BreakVector _location))
  ;[1 1 1] Play sound if player is in range and presses (Use)
  (:Pressed
    (if (Collision|IsOverlappingActor (Variables|Default|GetTrigger%20Box) (Game|GetPlayerCharacter 0) :!class /Script/Engine.PrimitiveComponent)
      (bind _newtrack_0 (Timeline|Timeline_0 PlayFromStart)
        (:Update
          (Transformation|SetRelativeLocation _button (Math|Vector|MakeVector _x _newtrack_0 _z) false false))
        (:Finished
          (Audio|PlaySoundatLocation (Variables|Default|GetSound) (Transformation|GetWorldLocation (Variables|Default|GetBase)))
          (Default|CallButtonPressed))))))

(fn ConstructionScript)