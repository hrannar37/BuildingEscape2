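; Portal prop that teleports any actor overlapping its Portal component to a linked OutPortal.
; The destination location and rotation come from the first child actor of OutPortal.
; For the player character, it also sets the controller's control rotation to match the exit.
; A timeline started on BeginPlay drives the Ring's relative rotation, which is applied every Tick.
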(event OnComponentBeginOverlap(Portal)
  (params (OverlappedComponent :type Primitive%20Component%20Object%20Reference) (OtherActor :type Actor%20Object%20Reference) (OtherComp :type Primitive%20Component%20Object%20Reference) (OtherBodyIndex :type Integer) (bFromSweep :type Boolean) (SweepResult :type Hit%20Result%20Structure%20%28by%20ref%29))
  (bind _returnvalue (Game|GetPlayerCharacter 0))
  (bind _out_portal (Variables|Default|GetOut%20Portal))
  (bind _childactors (Actor|GetAllChildActors _out_portal true))
  (bind _output (Utilities|Array|Get(acopy) _childactors))
  (bind _returnvalue_2 (Transformation|GetActorRotation _output))
  ;[1 1 1] Teleporting the overlapped object
  (Transformation|Teleport OtherActor (Transformation|GetActorLocation _output) _returnvalue_2)
  (if (== OtherActor _returnvalue)
    (Pawn|SetControlRotation (Pawn|GetController _returnvalue) _returnvalue_2)))

(event EventBeginPlay
  ;[1 1 1] Rotates the portal ring
  (bind (_direction _newtrack_0 _newtrack_1 _newtrack_2) (Timeline|Timeline_0 Play)))

(event EventTick
  (params (DeltaSeconds :type Float%20%28single-precision%29))
  ;[1 1 1] Rotates the portal ring
  (Transformation|SetRelativeRotation (Variables|Default|GetRing) (Math|Rotator|MakeRotator (stale EventBeginPlay _newtrack_1) (stale EventBeginPlay _newtrack_0) (stale EventBeginPlay _newtrack_2)) false false))

(fn ConstructionScript)