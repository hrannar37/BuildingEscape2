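; Runs a Lights Out-style puzzle on a 5x5 grid of trigger and plate pairs.
; Each cell is a reused state-change node that handles Use input and passes switches to its orthogonal neighbours.
; A setup node on Tick sends initial states from one of seven GameSetup variants, or flashes random cells as a disco floor while the game is not started.
; Use input also sets GameWon when all cells share one state.
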(event EventBeginPlay
  (Input|EnableInput (Game|GetPlayerController 0)))

(event Collision|EventActorBeginOverlap
  (params (OtherActor :type Actor%20Object%20Reference)))

(event EventTick
  (params (DeltaSeconds :type Float%20%28single-precision%29))
  (Utilities|InitialSetupANDDiscoFloor
    (:InitialSetupA1
      (Utilities|PlayerInteractionANDStateChange (Variables|Default|GetTrigger%20A1) (Variables|Default|GetPlate%20A1) (Variables|Default|GetGameSetupA1)) ; enters at Initial State
    )
    (:InitialSetupA2
      (Utilities|PlayerInteractionANDStateChange (Variables|Default|GetTrigger%20A2) (Variables|Default|GetPlate%20A2) (Variables|Default|GetGameSetupA2)) ; enters at Initial State
    )
    (:InitialSetupA3
      (Utilities|PlayerInteractionANDStateChange (Variables|Default|GetTrigger%20A3) (Variables|Default|GetPlate%20A3) (Variables|Default|GetGameSetupA3)) ; enters at Initial State
    )
    (:InitialSetupA4
      (Utilities|PlayerInteractionANDStateChange (Variables|Default|GetTrigger%20A4) (Variables|Default|GetPlate%20A4) (Variables|Default|GetGameSetupA4)) ; enters at Initial State
    )
    (:InitialSetupA5
      (Utilities|PlayerInteractionANDStateChange (Variables|Default|GetTrigger%20A5) (Variables|Default|GetPlate%20A5) (Variables|Default|GetGameSetupA5)) ; enters at Initial State
    )
    (:InitialSetupB1
      (Utilities|PlayerInteractionANDStateChange (Variables|Default|GetTrigger%20B1) (Variables|Default|GetPlate%20B1) (Variables|Default|GetGameSetupB1)) ; enters at Initial State
    )
    (:InitialSetupB2
      (Utilities|PlayerInteractionANDStateChange (Variables|Default|GetTrigger%20B2) (Variables|Default|GetPlate%20B2) (Variables|Default|GetGameSetupB2)) ; enters at Initial State
    )
    (:InitialSetupB3
      (Utilities|PlayerInteractionANDStateChange (Variables|Default|GetTrigger%20B3) (Variables|Default|GetPlate%20B3) (Variables|Default|GetGameSetupB3)) ; enters at Initial State
    )
    (:InitialSetupB4
      (Utilities|PlayerInteractionANDStateChange (Variables|Default|GetTrigger%20B4) (Variables|Default|GetPlate%20B4) (Variables|Default|GetGameSetupB4)) ; enters at Initial State
    )
    (:InitialSetupB5
      (Utilities|PlayerInteractionANDStateChange (Variables|Default|GetTrigger%20B5) (Variables|Default|GetPlate%20B5) (Variables|Default|GetGameSetupB5)) ; enters at Initial State
    )
    (:InitialSetupC1
      (Utilities|PlayerInteractionANDStateChange (Variables|Default|GetTrigger%20C1) (Variables|Default|GetPlate%20C1) (Variables|Default|GetGameSetupC1)) ; enters at Initial State
    )
    (:InitialSetupC2
      (Utilities|PlayerInteractionANDStateChange (Variables|Default|GetTrigger%20C2) (Variables|Default|GetPlate%20C2) (Variables|Default|GetGameSetupC2)) ; enters at Initial State
    )
    (:InitialSetupC3
      (Utilities|PlayerInteractionANDStateChange (Variables|Default|GetTrigger%20C3) (Variables|Default|GetPlate%20C3) (Variables|Default|GetGameSetupC3)) ; enters at Initial State
    )
    (:InitialSetupC4
      (Utilities|PlayerInteractionANDStateChange (Variables|Default|GetTrigger%20C4) (Variables|Default|GetPlate%20C4) (Variables|Default|GetGameSetupC4)) ; enters at Initial State
    )
    (:InitialSetupC5
      (Utilities|PlayerInteractionANDStateChange (Variables|Default|GetTrigger%20C5) (Variables|Default|GetPlate%20C5) (Variables|Default|GetGameSetupC5)) ; enters at Initial State
    )
    (:InitialSetupD1
      (Utilities|PlayerInteractionANDStateChange (Variables|Default|GetTrigger%20D1) (Variables|Default|GetPlate%20D1) (Variables|Default|GetGameSetupD1)) ; enters at Initial State
    )
    (:InitialSetupD2
      (Utilities|PlayerInteractionANDStateChange (Variables|Default|GetTrigger%20D2) (Variables|Default|GetPlate%20D2) (Variables|Default|GetGameSetupD2)) ; enters at Initial State
    )
    (:InitialSetupD3
      (Utilities|PlayerInteractionANDStateChange (Variables|Default|GetTrigger%20D3) (Variables|Default|GetPlate%20D3) (Variables|Default|GetGameSetupD3)) ; enters at Initial State
    )
    (:InitialSetupD4
      (Utilities|PlayerInteractionANDStateChange (Variables|Default|GetTrigger%20D4) (Variables|Default|GetPlate%20D4) (Variables|Default|GetGameSetupD4)) ; enters at Initial State
    )
    (:InitialSetupD5
      (Utilities|PlayerInteractionANDStateChange (Variables|Default|GetTrigger%20D5) (Variables|Default|GetPlate%20D5) (Variables|Default|GetGameSetupD5)) ; enters at Initial State
    )
    (:InitialSetupE1
      (Utilities|PlayerInteractionANDStateChange (Variables|Default|GetTrigger%20E1) (Variables|Default|GetPlate%20E1) (Variables|Default|GetGameSetupE1)) ; enters at Initial State
    )
    (:InitialSetupE2
      (Utilities|PlayerInteractionANDStateChange (Variables|Default|GetTrigger%20E2) (Variables|Default|GetPlate%20E2) (Variables|Default|GetGameSetupE2)) ; enters at Initial State
    )
    (:InitialSetupE3
      (Utilities|PlayerInteractionANDStateChange (Variables|Default|GetTrigger%20E3) (Variables|Default|GetPlate%20E3) (Variables|Default|GetGameSetupE3)) ; enters at Initial State
    )
    (:InitialSetupE4
      (Utilities|PlayerInteractionANDStateChange (Variables|Default|GetTrigger%20E4) (Variables|Default|GetPlate%20E4) (Variables|Default|GetGameSetupE4)) ; enters at Initial State
    )
    (:InitialSetupE5
      (Utilities|PlayerInteractionANDStateChange (Variables|Default|GetTrigger%20E5) (Variables|Default|GetPlate%20E5) (Variables|Default|GetGameSetupE5)) ; enters at Initial State
    )
    (:DiscoFloorA1
      (Utilities|PlayerInteractionANDStateChange (Variables|Default|GetTrigger%20A1) (Variables|Default|GetPlate%20A1) (Variables|Default|GetGameSetupA1)) ; enters at Disco Floor
    )
    (:DiscoFloorA2
      (Utilities|PlayerInteractionANDStateChange (Variables|Default|GetTrigger%20A2) (Variables|Default|GetPlate%20A2) (Variables|Default|GetGameSetupA2)) ; enters at Disco Floor
    )
    (:DiscoFloorA3
      (Utilities|PlayerInteractionANDStateChange (Variables|Default|GetTrigger%20A3) (Variables|Default|GetPlate%20A3) (Variables|Default|GetGameSetupA3)) ; enters at Disco Floor
    )
    (:DiscoFloorA4
      (Utilities|PlayerInteractionANDStateChange (Variables|Default|GetTrigger%20A4) (Variables|Default|GetPlate%20A4) (Variables|Default|GetGameSetupA4)) ; enters at Disco Floor
    )
    (:DiscoFloorA5
      (Utilities|PlayerInteractionANDStateChange (Variables|Default|GetTrigger%20A5) (Variables|Default|GetPlate%20A5) (Variables|Default|GetGameSetupA5)) ; enters at Disco Floor
    )
    (:DiscoFloorB1
      (Utilities|PlayerInteractionANDStateChange (Variables|Default|GetTrigger%20B1) (Variables|Default|GetPlate%20B1) (Variables|Default|GetGameSetupB1)) ; enters at Disco Floor
    )
    (:DiscoFloorB2
      (Utilities|PlayerInteractionANDStateChange (Variables|Default|GetTrigger%20B2) (Variables|Default|GetPlate%20B2) (Variables|Default|GetGameSetupB2)) ; enters at Disco Floor
    )
    (:DiscoFloorB3
      (Utilities|PlayerInteractionANDStateChange (Variables|Default|GetTrigger%20B3) (Variables|Default|GetPlate%20B3) (Variables|Default|GetGameSetupB3)) ; enters at Disco Floor
    )
    (:DiscoFloorB4
      (Utilities|PlayerInteractionANDStateChange (Variables|Default|GetTrigger%20B4) (Variables|Default|GetPlate%20B4) (Variables|Default|GetGameSetupB4)) ; enters at Disco Floor
    )
    (:DiscoFloorB5
      (Utilities|PlayerInteractionANDStateChange (Variables|Default|GetTrigger%20B5) (Variables|Default|GetPlate%20B5) (Variables|Default|GetGameSetupB5)) ; enters at Disco Floor
    )
    (:DiscoFloorC1
      (Utilities|PlayerInteractionANDStateChange (Variables|Default|GetTrigger%20C1) (Variables|Default|GetPlate%20C1) (Variables|Default|GetGameSetupC1)) ; enters at Disco Floor
    )
    (:DiscoFloorC2
      (Utilities|PlayerInteractionANDStateChange (Variables|Default|GetTrigger%20C2) (Variables|Default|GetPlate%20C2) (Variables|Default|GetGameSetupC2)) ; enters at Disco Floor
    )
    (:DiscoFloorC3
      (Utilities|PlayerInteractionANDStateChange (Variables|Default|GetTrigger%20C3) (Variables|Default|GetPlate%20C3) (Variables|Default|GetGameSetupC3)) ; enters at Disco Floor
    )
    (:DiscoFloorC4
      (Utilities|PlayerInteractionANDStateChange (Variables|Default|GetTrigger%20C4) (Variables|Default|GetPlate%20C4) (Variables|Default|GetGameSetupC4)) ; enters at Disco Floor
    )
    (:DiscoFloorC5
      (Utilities|PlayerInteractionANDStateChange (Variables|Default|GetTrigger%20C5) (Variables|Default|GetPlate%20C5) (Variables|Default|GetGameSetupC5)) ; enters at Disco Floor
    )
    (:DiscoFloorD1
      (Utilities|PlayerInteractionANDStateChange (Variables|Default|GetTrigger%20D1) (Variables|Default|GetPlate%20D1) (Variables|Default|GetGameSetupD1)) ; enters at Disco Floor
    )
    (:DiscoFloorD2
      (Utilities|PlayerInteractionANDStateChange (Variables|Default|GetTrigger%20D2) (Variables|Default|GetPlate%20D2) (Variables|Default|GetGameSetupD2)) ; enters at Disco Floor
    )
    (:DiscoFloorD3
      (Utilities|PlayerInteractionANDStateChange (Variables|Default|GetTrigger%20D3) (Variables|Default|GetPlate%20D3) (Variables|Default|GetGameSetupD3)) ; enters at Disco Floor
    )
    (:DiscoFloorD4
      (Utilities|PlayerInteractionANDStateChange (Variables|Default|GetTrigger%20D4) (Variables|Default|GetPlate%20D4) (Variables|Default|GetGameSetupD4)) ; enters at Disco Floor
    )
    (:DiscoFloorD5
      (Utilities|PlayerInteractionANDStateChange (Variables|Default|GetTrigger%20D5) (Variables|Default|GetPlate%20D5) (Variables|Default|GetGameSetupD5)) ; enters at Disco Floor
    )
    (:DiscoFloorE1
      (Utilities|PlayerInteractionANDStateChange (Variables|Default|GetTrigger%20E1) (Variables|Default|GetPlate%20E1) (Variables|Default|GetGameSetupE1)) ; enters at Disco Floor
    )
    (:DiscoFloorE2
      (Utilities|PlayerInteractionANDStateChange (Variables|Default|GetTrigger%20E2) (Variables|Default|GetPlate%20E2) (Variables|Default|GetGameSetupE2)) ; enters at Disco Floor
    )
    (:DiscoFloorE3
      (Utilities|PlayerInteractionANDStateChange (Variables|Default|GetTrigger%20E3) (Variables|Default|GetPlate%20E3) (Variables|Default|GetGameSetupE3)) ; enters at Disco Floor
    )
    (:DiscoFloorE4
      (Utilities|PlayerInteractionANDStateChange (Variables|Default|GetTrigger%20E4) (Variables|Default|GetPlate%20E4) (Variables|Default|GetGameSetupE4)) ; enters at Disco Floor
    )
    (:DiscoFloorE5
      (Utilities|PlayerInteractionANDStateChange (Variables|Default|GetTrigger%20E5) (Variables|Default|GetPlate%20E5) (Variables|Default|GetGameSetupE5)) ; enters at Disco Floor
    )))

(event Input|ActionEvents|InputActionUse
  (params (Key :type Key%20Structure))
  (:Pressed
    (Utilities|PlayerInteractionANDStateChange (Variables|Default|GetTrigger%20C2) (Variables|Default|GetPlate%20C2) (Variables|Default|GetGameSetupC2)) ; enters at Use Input
  ))

(event Input|ActionEvents|InputActionUse
  (params (Key :type Key%20Structure))
  (:Pressed
    (Utilities|PlayerInteractionANDStateChange (Variables|Default|GetTrigger%20C3) (Variables|Default|GetPlate%20C3) (Variables|Default|GetGameSetupC3)) ; enters at Use Input
  ))

(event Input|ActionEvents|InputActionUse
  (params (Key :type Key%20Structure))
  (:Pressed
    (Utilities|PlayerInteractionANDStateChange (Variables|Default|GetTrigger%20C4) (Variables|Default|GetPlate%20C4) (Variables|Default|GetGameSetupC4)) ; enters at Use Input
  ))

(event Input|ActionEvents|InputActionUse
  (params (Key :type Key%20Structure))
  (:Pressed
    (Utilities|PlayerInteractionANDStateChange (Variables|Default|GetTrigger%20C5) (Variables|Default|GetPlate%20C5) (Variables|Default|GetGameSetupC5)) ; enters at Use Input
  ))

(event Input|ActionEvents|InputActionUse
  (params (Key :type Key%20Structure))
  (:Pressed
    (Utilities|PlayerInteractionANDStateChange (Variables|Default|GetTrigger%20D1) (Variables|Default|GetPlate%20D1) (Variables|Default|GetGameSetupD1)) ; enters at Use Input
  ))

(event Input|ActionEvents|InputActionUse
  (params (Key :type Key%20Structure))
  (:Pressed
    (Utilities|PlayerInteractionANDStateChange (Variables|Default|GetTrigger%20D2) (Variables|Default|GetPlate%20D2) (Variables|Default|GetGameSetupD2)) ; enters at Use Input
  ))

(event Input|ActionEvents|InputActionUse
  (params (Key :type Key%20Structure))
  (:Pressed
    (Utilities|PlayerInteractionANDStateChange (Variables|Default|GetTrigger%20D3) (Variables|Default|GetPlate%20D3) (Variables|Default|GetGameSetupD3)) ; enters at Use Input
  ))

(event Input|ActionEvents|InputActionUse
  (params (Key :type Key%20Structure))
  (:Pressed
    (Utilities|PlayerInteractionANDStateChange (Variables|Default|GetTrigger%20D4) (Variables|Default|GetPlate%20D4) (Variables|Default|GetGameSetupD4)) ; enters at Use Input
  ))

(event Input|ActionEvents|InputActionUse
  (params (Key :type Key%20Structure))
  (:Pressed
    (Utilities|PlayerInteractionANDStateChange (Variables|Default|GetTrigger%20D5) (Variables|Default|GetPlate%20D5) (Variables|Default|GetGameSetupD5)) ; enters at Use Input
  ))

(event Input|ActionEvents|InputActionUse
  (params (Key :type Key%20Structure))
  (:Pressed
    (Utilities|PlayerInteractionANDStateChange (Variables|Default|GetTrigger%20E1) (Variables|Default|GetPlate%20E1) (Variables|Default|GetGameSetupE1)) ; enters at Use Input
  ))

(event Input|ActionEvents|InputActionUse
  (params (Key :type Key%20Structure))
  (:Pressed
    (Utilities|PlayerInteractionANDStateChange (Variables|Default|GetTrigger%20E2) (Variables|Default|GetPlate%20E2) (Variables|Default|GetGameSetupE2)) ; enters at Use Input
  ))

(event Input|ActionEvents|InputActionUse
  (params (Key :type Key%20Structure))
  (:Pressed
    (Utilities|PlayerInteractionANDStateChange (Variables|Default|GetTrigger%20E3) (Variables|Default|GetPlate%20E3) (Variables|Default|GetGameSetupE3)) ; enters at Use Input
  ))

(event Input|ActionEvents|InputActionUse
  (params (Key :type Key%20Structure))
  (:Pressed
    (Utilities|PlayerInteractionANDStateChange (Variables|Default|GetTrigger%20E4) (Variables|Default|GetPlate%20E4) (Variables|Default|GetGameSetupE4)) ; enters at Use Input
  ))

(event Input|ActionEvents|InputActionUse
  (params (Key :type Key%20Structure))
  (:Pressed
    (Utilities|InitialSetupANDDiscoFloor) ; enters at UseInput
  ))

(event Input|ActionEvents|InputActionUse
  (params (Key :type Key%20Structure))
  (:Pressed
    (Utilities|PlayerInteractionANDStateChange (Variables|Default|GetTrigger%20A2) (Variables|Default|GetPlate%20A2) (Variables|Default|GetGameSetupA2)) ; enters at Use Input
  ))

(event Input|ActionEvents|InputActionUse
  (params (Key :type Key%20Structure))
  (:Pressed
    (Utilities|PlayerInteractionANDStateChange (Variables|Default|GetTrigger%20A3) (Variables|Default|GetPlate%20A3) (Variables|Default|GetGameSetupA3)) ; enters at Use Input
  ))

(event Input|ActionEvents|InputActionUse
  (params (Key :type Key%20Structure))
  (:Pressed
    (Utilities|PlayerInteractionANDStateChange (Variables|Default|GetTrigger%20A4) (Variables|Default|GetPlate%20A4) (Variables|Default|GetGameSetupA4)) ; enters at Use Input
  ))

(event Input|ActionEvents|InputActionUse
  (params (Key :type Key%20Structure))
  (:Pressed
    (Utilities|PlayerInteractionANDStateChange (Variables|Default|GetTrigger%20B4) (Variables|Default|GetPlate%20B4) (Variables|Default|GetGameSetupB4)) ; enters at Use Input
  ))

(event Input|ActionEvents|InputActionUse
  (params (Key :type Key%20Structure))
  (:Pressed
    (Utilities|PlayerInteractionANDStateChange (Variables|Default|GetTrigger%20A5) (Variables|Default|GetPlate%20A5) (Variables|Default|GetGameSetupA5)) ; enters at Use Input
  ))

(event Input|ActionEvents|InputActionUse
  (params (Key :type Key%20Structure))
  (:Pressed
    (Utilities|PlayerInteractionANDStateChange (Variables|Default|GetTrigger%20A1) (Variables|Default|GetPlate%20A1) (Variables|Default|GetGameSetupA1)) ; enters at Use Input
  ))

(event Input|ActionEvents|InputActionUse
  (params (Key :type Key%20Structure))
  (:Pressed
    (Utilities|PlayerInteractionANDStateChange (Variables|Default|GetTrigger%20B1) (Variables|Default|GetPlate%20B1) (Variables|Default|GetGameSetupB1)) ; enters at Use Input
  ))

(event Input|ActionEvents|InputActionUse
  (params (Key :type Key%20Structure))
  (:Pressed
    (Utilities|PlayerInteractionANDStateChange (Variables|Default|GetTrigger%20B2) (Variables|Default|GetPlate%20B2) (Variables|Default|GetGameSetupB2)) ; enters at Use Input
  ))

(event Input|ActionEvents|InputActionUse
  (params (Key :type Key%20Structure))
  (:Pressed
    (Utilities|PlayerInteractionANDStateChange (Variables|Default|GetTrigger%20B3) (Variables|Default|GetPlate%20B3) (Variables|Default|GetGameSetupB3)) ; enters at Use Input
  ))

(event Input|ActionEvents|InputActionUse
  (params (Key :type Key%20Structure))
  (:Pressed
    (Variables|Default|SetGameWon (or (Math|Boolean|ANDBoolean (stale _on_off) (stale _on_off) (stale _on_off) (stale _on_off) (stale _on_off) (stale _on_off) (stale _on_off) (stale _on_off) (stale _on_off) (stale _on_off) (stale _on_off) (stale _on_off) (stale _on_off) (stale _on_off) (stale _on_off) (stale _on_off) (stale _on_off) (stale _on_off) (stale _on_off) (stale _on_off) (stale _on_off) (stale _on_off) (stale _on_off) (stale _on_off) (stale _on_off)) (not (Math|Boolean|ORBoolean (stale _on_off) (stale _on_off) (stale _on_off) (stale _on_off) (stale _on_off) (stale _on_off) (stale _on_off) (stale _on_off) (stale _on_off) (stale _on_off) (stale _on_off) (stale _on_off) (stale _on_off) (stale _on_off) (stale _on_off) (stale _on_off) (stale _on_off) (stale _on_off) (stale _on_off) (stale _on_off) (stale _on_off) (stale _on_off) (stale _on_off) (stale _on_off) (stale _on_off)))))))

(event Input|ActionEvents|InputActionUse
  (params (Key :type Key%20Structure))
  (:Pressed
    (Utilities|PlayerInteractionANDStateChange (Variables|Default|GetTrigger%20B5) (Variables|Default|GetPlate%20B5) (Variables|Default|GetGameSetupB5)) ; enters at Use Input
  ))

(event Input|ActionEvents|InputActionUse
  (params (Key :type Key%20Structure))
  (:Pressed
    (Utilities|PlayerInteractionANDStateChange (Variables|Default|GetTrigger%20E5) (Variables|Default|GetPlate%20E5) (Variables|Default|GetGameSetupE5)) ; enters at Use Input
  ))

(event Input|ActionEvents|InputActionUse
  (params (Key :type Key%20Structure))
  (:Pressed
    (Utilities|PlayerInteractionANDStateChange (Variables|Default|GetTrigger%20C1) (Variables|Default|GetPlate%20C1) (Variables|Default|GetGameSetupC1)) ; enters at Use Input
  ))

(fn ConstructionScript)