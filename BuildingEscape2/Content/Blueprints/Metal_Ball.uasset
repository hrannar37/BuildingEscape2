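; Metal_Ball is an unfinished actor Blueprint with a Sphere component, apparently an experiment in making a ball stick to the surface below it.
; Each Tick it line-traces 500 units straight down on the Visibility channel with persistent debug drawing, and does nothing with the result.
; An impulse on the sphere, a Sticky-scaled impact-point calculation, a branch and an empty macro are left unconnected, and the custom event is empty.
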(event Custom|NiBBa)

(event EventBeginPlay)

(event Collision|EventActorBeginOverlap
  (params (OtherActor :type Actor%20Object%20Reference)))

(event EventTick
  (params (DeltaSeconds :type Float%20%28single-precision%29))
  (bind _returnvalue (Transformation|GetActorLocation))
  (Collision|LineTraceByChannel _returnvalue (- _returnvalue "0,0.000000,500.000000") "TraceTypeQuery1" false 0 "Persistent"))

(fn ConstructionScript)